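; BP_CamPlayer is a player camera pawn with yaw-relative movement, mouse look and spring-arm zoom.
; The mouse wheel sets a clamped target boom length that the axis event interpolates toward.
; Mouse look applies a deadzone and gates pitch input against an upper limit.
; CaptureCam hands spring arm rotation to or from control rotation on press or release, returning whether it still nearly matches the rotation saved on press.
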(event Input|AxisEvents|InputAxisMoveForward
  (params (AxisValue :type Float%20%28single-precision%29))
  ;[1 1 1] Controling camera
  (Pawn|Input|AddMovementInput (Math|Vector|GetForwardVector (Math|Rotator|MakeRotator 0.0 0.0 (.yaw (Pawn|GetControlRotation :!class /Script/Engine.Pawn)))) AxisValue false))

(event Input|AxisEvents|InputAxisMoveRight
  (params (AxisValue :type Float%20%28single-precision%29))
  ;[1 1 1] Controling camera
  (Pawn|Input|AddMovementInput (Math|Vector|GetRightVector (Math|Rotator|MakeRotator 0.0 0.0 (.yaw (Pawn|GetControlRotation :!class /Script/Engine.Pawn)))) AxisValue false))

(event Input|MouseEvents|MouseWheelAxis
  (params (AxisValue :type Float%20%28single-precision%29))
  ;[1 1 1] Controling camera
  (Variables|/Script/Engine.SpringArmComponent|SetTargetArmLength (Variables|Default|GetSpringArm) (Math|Float|Clamp(Float) (Math|Interpolation|FInterpTo (Variables|/Script/Engine.SpringArmComponent|GetTargetArmLength (Variables|Default|GetSpringArm)) (Variables|Default|GetCamBoomLength) (Utilities|Time|GetWorldDeltaSeconds) 5.0) 3e+02 2e+03)))

(event Input|MouseEvents|MouseX
  (params (AxisValue :type Float%20%28single-precision%29))
  ;[1 1 1] Controling camera
  (if (> (Math|Float|Absolute(Float) AxisValue) 0.1)
    (Pawn|Input|AddControllerYawInput AxisValue)))

(event Input|MouseEvents|MouseY
  (params (AxisValue :type Float%20%28single-precision%29))
  (bind _returnvalue (Math|Float|Clamp(Float) AxisValue -2.0 2.0))
  ;[1 1 1] Controling camera
  (if (> (Math|Float|Absolute(Float) AxisValue) 0.1)
    (Math|Float|CompareFloat (+ (Math|Float|Clamp(Float) (.pitch (Pawn|GetControlRotation :!class /Script/Engine.Pawn)) 2.7e+02 3.5e+02) _returnvalue) 3.5e+02
      (:==
        _)
      (:<
        _))
    (Pawn|Input|AddControllerPitchInput (* _returnvalue -1.0))))

(event Input|MouseEvents|MouseWheelDown
  (params (Key :type Key%20Structure :default "None"))
  ;[1 1 1] Controling camera
  (:Pressed
    (Variables|Default|SetCamBoomLength (Math|Float|Clamp(Float) (+ (Variables|/Script/Engine.SpringArmComponent|GetTargetArmLength (Variables|Default|GetSpringArm)) 3e+02) 3e+02 2e+03))))

(event Input|MouseEvents|MouseWheelUp
  (params (Key :type Key%20Structure :default "None"))
  ;[1 1 1] Controling camera
  (:Pressed
    (Variables|Default|SetCamBoomLength (Math|Float|Clamp(Float) (- (Variables|/Script/Engine.SpringArmComponent|GetTargetArmLength (Variables|Default|GetSpringArm)) 3e+02) 3e+02 2e+03))))

(fn ConstructionScript)

(fn CaptureCam
  (params (Pressed/Realeased :type Boolean))
  (if Pressed/Realeased
    (Variables|Default|SetLastRotationCam (Transformation|GetWorldRotation (Variables|Default|GetSpringArm)))
    (Pawn|SetControlRotation (Game|GetPlayerController 0) (Transformation|GetWorldRotation (Variables|Default|GetSpringArm)))
    (Variables|/Script/Engine.SpringArmComponent|SetbUsePawnControlRotation (Variables|Default|GetSpringArm) true)
    (else
      (Transformation|SetWorldRotation (Variables|Default|GetSpringArm) (Pawn|GetControlRotation :!class /Script/Engine.Pawn) false false)
      (Variables|/Script/Engine.SpringArmComponent|SetbUsePawnControlRotation (Variables|Default|GetSpringArm) false)))
  (return (Math|Rotator|Equal(Rotator) (Variables|Default|GetLastRotationCam) (Transformation|GetWorldRotation (Variables|Default|GetSpringArm)) 0.1)))