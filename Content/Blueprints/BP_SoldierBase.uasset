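; Base soldier unit for an RTS-style game that moves on orders, attacks opposing-side pawns and takes damage.
; Move uses AIMoveTo toward a location or target actor, and PawnSensing sightings of enemies stop movement and start attacking.
; A looping timer rechecks the target, turning to face it or chasing it again when out of sight radius.
; At zero life it ragdolls, leaves the local player's selection and HUD, then is destroyed after a delay.
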(event OnSeePawn(PawnSensing)
  (params (Pawn :type Pawn%20Object%20Reference))
  ;[1 1 1] Attack enemy
  (CallFunction|HandlerConditionAttack Pawn))

(event Custom|CheckDistanceToEnemy
  ;[1 1 1] Attack enemy
  (Variables|Default|GetTargetForAttack
    (:then
      (bind _status (Class|BPIAI|GetStatus(Message) (Variables|Default|GetTargetForAttack)))
      (if (Utilities|Enum|Equal(Enum) _status "NewEnumerator3")
        (Variables|Default|SetTargetForAttack 0)
        (Variables|Default|SetDoingStatus "NewEnumerator0")
        (Utilities|Time|ClearandInvalidateTimerbyHandle (Variables|Default|GetCheckEnemy))
        (elif (> (Math|Vector|Distance(Vector) (Transformation|GetActorLocation (Variables|Default|GetTargetForAttack)) (Transformation|GetActorLocation)) (Variables|Default|GetSight%20Radius))
          (Utilities|FlowControl|DoOnce false
            (:Completed
              (Variables|Default|SetDoingStatus "NewEnumerator0")
              (Default|Move self (Transformation|GetActorLocation (Variables|Default|GetTargetForAttack)) (Variables|Default|GetTargetForAttack))))
          (else
            (AI|Navigation|StopMovement (AI|GetAIController self))
            (Transformation|SetActorRotation (Math|Rotator|MakeRotator 0.0 0.0 (.yaw (Math|Rotator|FindLookatRotation (Transformation|GetActorLocation) (Transformation|GetActorLocation (Variables|Default|GetTargetForAttack))))))
            (Variables|Default|SetDoingStatus "NewEnumerator2")))))
    (:else
      (bind _enemyunit (Variables|Default|GetEnemyUnit)
        (:then
          (if (> (Math|Vector|Distance(Vector) (Transformation|GetActorLocation _enemyunit) (Transformation|GetActorLocation)) (Variables|Default|GetSight%20Radius))
            (Variables|Default|SetDoingStatus "NewEnumerator0")
            (Utilities|Time|ClearandInvalidateTimerbyHandle (Variables|Default|GetCheckEnemy))))
        (:else
          (Variables|Default|SetDoingStatus "NewEnumerator0")
          (Utilities|Time|ClearandInvalidateTimerbyHandle (Variables|Default|GetCheckEnemy)))))))

(event Custom|PursuitReset
  (bind _targetforattack (Variables|Default|GetTargetForAttack))
  ;[1 1 1] Attack enemy
  (Utilities|FlowControl|DoOnce false) ; enters at Reset
)

(event Game|Damage|EventAnyDamage
  (params (Damage :type Float%20%28single-precision%29) (DamageType :type Damage%20Type%20Object%20Reference) (InstigatedBy :type Controller%20Object%20Reference) (DamageCauser :type Actor%20Object%20Reference))
  ;[1 1 1] Attack enemy
  (bind _output_get (Variables|Default|SetLife (Math|Float|Clamp(Float) (- (Variables|Default|GetLife) Damage) 0.0 (Variables|Default|GetLife))))
  (if (== _output_get 0.0)
    (Utilities|FlowControl|DoOnce false
      (:Completed
        (CallFunction|PreparetoDestroy)
        (Utilities|FlowControl|Delay 3.0)
        (Actor|DestroyActor)))))

(event EventMove
  (params (MoveToLocation :type Vector :default "0, 0, 0") (TargetForAttack :type Actor%20Object%20Reference))
  (CallFunction|PursuitReset)
  (Utilities|IsValid TargetForAttack
    (:Is%20Valid
      (Variables|Default|SetTargetForAttack TargetForAttack)
      (Class|PawnSensingComponent|SetSensingInterval (Variables|Default|GetPawnSensing) 0.1)
      (bind _movementresult (AI|AIMoveTo self "0, 0, 0" (Variables|Default|GetTargetForAttack) 5.0 false)
        (:then
          (switch Utilities|FlowControl|Switch|SwitchonEPathFollowingResult _movementresult
            (:Success
              (Variables|Default|SetDoingStatus "NewEnumerator1")
              (Utilities|IsValid (Variables|Default|GetTargetForAttack)
                (:Is%20Valid
                  (bind _returnvalue (Utilities|Time|SetTimerbyEvent (EventDispatchers|CreateEvent self :!event Custom|CheckDistanceToEnemy) 0.5 true))
                  (Variables|Default|SetCheckEnemy _returnvalue))))
            (:Aborted
              (Variables|Default|SetDoingStatus "NewEnumerator1"))))
        (:OnSuccess
          (switch Utilities|FlowControl|Switch|SwitchonEPathFollowingResult _movementresult
            (:Success
              (Variables|Default|SetDoingStatus "NewEnumerator0"))))
        (:OnFail
          (switch Utilities|FlowControl|Switch|SwitchonEPathFollowingResult _movementresult
            (:Aborted
              (Variables|Default|SetDoingStatus "NewEnumerator1"))))))
    (:Is%20Not%20Valid
      (Variables|Default|SetTargetForAttack 0)
      (bind _movementresult_2 (AI|AIMoveTo self MoveToLocation 0 5.0 false)
        (:then
          (switch Utilities|FlowControl|Switch|SwitchonEPathFollowingResult _movementresult_2
            (:Success
              (Variables|Default|SetDoingStatus "NewEnumerator1"))
            (:Aborted
              (Variables|Default|SetDoingStatus "NewEnumerator1"))))
        (:OnSuccess
          (switch Utilities|FlowControl|Switch|SwitchonEPathFollowingResult _movementresult_2
            (:Success
              (Variables|Default|SetDoingStatus "NewEnumerator0"))))))))

(fn ConstructionScript
  (Transformation|AttachComponentToComponent (Variables|Default|GetStaticMesh4) (Variables|Character|GetMesh) "hand_rSocket" "SnapToTarget" "SnapToTarget" "SnapToTarget" true)
  (Transformation|AttachComponentToComponent (Variables|Default|GetStaticMesh) (Variables|Character|GetMesh) "c_skull_03_xSocket" "SnapToTarget" "SnapToTarget" "SnapToTarget" true)
  (Variables|/Script/AIModule.PawnSensingComponent|SetSightRadius (Variables|Default|GetPawnSensing) (Variables|Default|GetSight%20Radius)))

(fn HandlerConditionAttack
  (params (FoundPawn :type Actor%20Object%20Reference))
  (bind _sidewar (Class|BPIAI|GetSideWar(Message) FoundPawn))
  (if (Utilities|Enum|NotEqual(Enum) _sidewar (Variables|Default|GetSideWar))
    (Variables|Default|SetEnemyUnit FoundPawn)
    (Utilities|IsValid (Variables|Default|GetTargetForAttack)
      (:Is%20Valid
        (if (== (Variables|Default|GetEnemyUnit) (Variables|Default|GetTargetForAttack))
          (Class|PawnSensingComponent|SetSensingInterval (Variables|Default|GetPawnSensing) 0.5)
          (switch Utilities|FlowControl|Switch|SwitchonE_DoingStatus (Variables|Default|GetDoingStatus) :!label _label
            (:NewEnumerator0
              _)
            (:NewEnumerator1
              (Utilities|IsValid (Variables|Default|GetTargetForAttack)
                (:Is%20Valid
                  (AI|Navigation|StopMovement (AI|GetAIController self)))))
            (:NewEnumerator2
              _))
          (Transformation|SetActorRotation (Math|Rotator|FindLookatRotation (Transformation|GetActorLocation) (Transformation|GetActorLocation (Variables|Default|GetEnemyUnit))))
          (Variables|Default|SetDoingStatus "NewEnumerator2")
          (bind _returnvalue (Utilities|Time|SetTimerbyEvent (EventDispatchers|CreateEvent self :!event Custom|CheckDistanceToEnemy) 0.5 true))
          (Variables|Default|SetCheckEnemy _returnvalue)))
      (:Is%20Not%20Valid
        (goto _label)))))

(fn PreparetoDestroy
  (Utilities|Time|ClearandInvalidateTimerbyHandle (Variables|Default|GetCheckEnemy))
  (AI|Navigation|StopMovement (AI|GetAIController self))
  (Variables|Default|SetDoingStatus "NewEnumerator3")
  (Components|DestroyComponent (Variables|Collision|GetCapsuleComponent))
  (Physics|SetSimulatePhysics (Variables|Character|GetMesh) true)
  (bind _playercontrollers (Class|BPIGameMode|GetPlayerControllersGM(Message) (Game|GetGameMode)))
  (bind _array_element (Utilities|Array|ForEachLoopwithBreak _playercontrollers :!label _label)
    (:LoopBody
      (if (Pawn|IsLocalController _array_element)
        (bind _selectedunits (Class|BPISelectionUnits|GetSelectedUnits(Message) _array_element))
        (Utilities|Array|RemoveItem _selectedunits self)
        (Class|BPISelectionUnits|SetSelectedUnits(Message) _array_element _selectedunits)
        (Class|BPISelectionUnits|Add/RemoveSelectUnitsfromHUD(Message) (HUD|GetHUD _array_element))
        (goto _label Break)))
    (:Completed
      (return))))

(fn GetSideWar
  (return (Variables|Default|GetSideWar)))

(fn GetStatus
  (return (Variables|Default|GetDoingStatus)))